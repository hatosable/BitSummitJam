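; BP_CheckPoint is a checkpoint trigger that registers itself with the game mode when the player reaches it.
; On the first Box overlap by player 0's pawn, it passes itself through SetCheckPointMessage and sets CheckOn so it only registers once.
; Every begin and end overlap also sends CloseLogselectMessage and OpenLogselectMessage, respectively, to the overlapping actor, whether or not it is the player.
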(event `self.Box.OnComponentBeginOverlap`
  (params (OverlappedComponent :type "PrimitiveComponent Object Reference") (OtherActor :type "Actor Object Reference") (OtherComp :type "PrimitiveComponent Object Reference") (OtherBodyIndex :type Integer) (bFromSweep :type Boolean) (SweepResult :type "HitResult Structure (by ref)"))
  (message `/Game/Player/IF_Player.CloseLogselect` OtherActor)
  (if (and (== OtherActor (`GameplayStatics.GetPlayerPawn` 0)) (not (`self.CheckOn`)))
    (message `/Game/System/IF_MainGameMode.SetCheckPoint` (`GameplayStatics.GetGameMode`) self)
    (set `self.CheckOn` true)))

(event `self.Box.OnComponentEndOverlap`
  (params (OverlappedComponent :type "PrimitiveComponent Object Reference") (OtherActor :type "Actor Object Reference") (OtherComp :type "PrimitiveComponent Object Reference") (OtherBodyIndex :type Integer))
  (message `/Game/Player/IF_Player.OpenLogselect` OtherActor))

(fn `UserConstructionScript`)