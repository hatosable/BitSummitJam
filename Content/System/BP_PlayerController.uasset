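; Player controller that relays player input to whatever control object the GameMode supplies.
; Move axis, jump press and release, left shoulder, and selection right, left, cancel and action inputs each call a matching message on GameMode's ControlObjectMessage, keeping gameplay response out of the controller.
; F1, F2 and F3 act as level shortcuts, opening the Title, Tutorial and Stage_1 maps directly.
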(event `InputAxis|Move`
  (params (AxisValue :type "Float (single-precision)"))
  (bind _controlobject (message `/Game/System/IF_MainGameMode.ControlObject` (`GameplayStatics.GetGameMode`)))
  (message `/Game/System/IF_Controler.AxisRight/Left` _controlobject AxisValue))

(event `InputAction|Jump`
  (params (Key :type "Key Structure"))
  (bind _returnvalue (`GameplayStatics.GetGameMode`))
  (:`Pressed`
    (bind _controlobject (message `/Game/System/IF_MainGameMode.ControlObject` _returnvalue))
    (message `/Game/System/IF_Controler.PressedA` _controlobject))
  (:`Released`
    (bind _controlobject_2 (message `/Game/System/IF_MainGameMode.ControlObject` _returnvalue))
    (message `/Game/System/IF_Controler.RelesedA` _controlobject_2)))

(event `InputAction|LeftShoulder`
  (params (Key :type "Key Structure"))
  (:`Pressed`
    (bind _controlobject (message `/Game/System/IF_MainGameMode.ControlObject` (`GameplayStatics.GetGameMode`)))
    (message `/Game/System/IF_Controler.LeftShoulder` _controlobject)))

(event `InputAction|SelectRight`
  (params (Key :type "Key Structure"))
  (:`Pressed`
    (bind _controlobject (message `/Game/System/IF_MainGameMode.ControlObject` (`GameplayStatics.GetGameMode`)))
    (message `/Game/System/IF_Controler.Right` _controlobject)))

(event `InputAction|SelectLeft`
  (params (Key :type "Key Structure"))
  (:`Pressed`
    (bind _controlobject (message `/Game/System/IF_MainGameMode.ControlObject` (`GameplayStatics.GetGameMode`)))
    (message `/Game/System/IF_Controler.Left` _controlobject)))

(event `InputAction|SelectCancel`
  (params (Key :type "Key Structure"))
  (:`Pressed`
    (bind _controlobject (message `/Game/System/IF_MainGameMode.ControlObject` (`GameplayStatics.GetGameMode`)))
    (message `/Game/System/IF_Controler.Cancel` _controlobject)))

(event `InputAction|SelectAction`
  (params (Key :type "Key Structure"))
  (:`Pressed`
    (bind _controlobject (message `/Game/System/IF_MainGameMode.ControlObject` (`GameplayStatics.GetGameMode`)))
    (message `/Game/System/IF_Controler.LogAction` _controlobject)))

(event `Key|F1`
  (params (Key :type "Key Structure"))
  (:`Pressed`
    (`GameplayStatics.OpenLevelBySoftObjectPtr` "/Game/Map/Production/Title.Title")))

(event `Key|F2`
  (params (Key :type "Key Structure"))
  (:`Pressed`
    (`GameplayStatics.OpenLevelBySoftObjectPtr` "/Game/Map/Production/Tutorial.Tutorial")))

(event `Key|F3`
  (params (Key :type "Key Structure"))
  (:`Pressed`
    (`GameplayStatics.OpenLevelBySoftObjectPtr` "/Game/Map/Production/Stage_1.Stage_1")))

(fn `UserConstructionScript`)