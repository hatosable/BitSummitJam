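; Player character Blueprint with single-axis movement and jump, which can sacrifice itself to leave a chosen "log effect" actor at its position.
; SelectAction opens a four-option WBP_LogSelect menu with time dilation at zero, while left/right cycle the index and Tick highlights it.
; Confirming disables movement, then after a delay destroys the player, spawns the chosen class and notifies the GameMode.
; E asks the GameMode to undo.
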(event `self.ReceiveBeginPlay`
  (bind _returnvalue (`|CreateWidget` "/Game/UI/WBP_LogSelect.WBP_LogSelect_C"))
  (bind _output_get (set `self.SkillUI` _returnvalue))
  (`UserWidget.AddToViewport` _output_get 0)
  (set `self.SelectWindow` (`|MakeArray` (`/Game/UI/WBP_LogSelect.LogEffect1` _output_get) (`/Game/UI/WBP_LogSelect.LogEffect2` _output_get) (`/Game/UI/WBP_LogSelect.LogEffect3` _output_get) (`/Game/UI/WBP_LogSelect.LogEffect4` _output_get))))

(event `self.ReceiveTick`
  (params (DeltaSeconds :type "Float (single-precision)"))
  (for (_array_element _array_index) (`self.SelectWindow`)
    (if (== _array_index (`self.Index`))
      (`Button.SetBackgroundColor` _array_element (struct :`R` 1.0 :`A` 1.0))
      (else
        (`Button.SetBackgroundColor` _array_element (struct :`R` 1.0 :`G` 1.0 :`B` 1.0 :`A` 1.0))))))

(event `InputAction|Jump`
  (params (Key :type "Key Structure"))
  ;[1 1 1] ジャンプ
  (:`Pressed`
    (if (not (`self.IsLogEffectSelect`))
      (`self.Jump`)))
  (:`Released`
    (`self.StopJumping`)))

(event `InputAxis|Move`
  (params (AxisValue :type "Float (single-precision)"))
  ;[1 1 1] 移動
  (if (not (`self.IsLogEffectSelect`))
    (`PawnMovementComponent.AddInputVector` (`self.CharacterMovement`) (`KismetMathLibrary.MakeVector` AxisValue) false)))

(event `InputAction|SelectAction`
  (params (Key :type "Key Structure"))
  (:`Pressed`
    (if (not (`self.IsDied`))
      (if (not (`self.IsLogEffectSelect`))
        ;[1 1 1] 効果選択メニュー表示
        (`self.F_ShowingSelectMenu`)
        (`GameplayStatics.SetGlobalTimeDilation` 0.0)
        (else
          ;[1 1 1] 効果決定
          (`|ExecutionSequence`
            (:`then_0`
              (set `self.IsLogEffectSelect` false)
              (set `self.IsDied` true)
              (`CharacterMovementComponent.DisableMovement` (`self.CharacterMovement`))
              (`GameplayStatics.SetGlobalTimeDilation` 1.0)
              (for _array_element (`self.SelectWindow`)
                (`Widget.SetVisibility` _array_element "Hidden")))
            (:`then_1`
              (`KismetSystemLibrary.Delay` 2.0)
              (`self.K2_DestroyActor`)
              (`|SpawnActorFromClass` (`|GetArrayItem` (`self.LofEffectLibrary`) (`self.Index`)) (`KismetMathLibrary.MakeTransform` (`self.K2_GetActorLocation`)) "Undefined" "OverrideRootScale" null null)
              (set `self.Index` 0)
              (message `/Game/System/IF_MainGameMode.IDUpdate` (`GameplayStatics.GetGameMode`)))))))))

(event `InputAction|SelectRight`
  (params (Key :type "Key Structure"))
  (:`Pressed`
    ;[1 1 1] 選択メニュー右送り
    (if (`self.IsLogEffectSelect`)
      (bind _result (`/Engine/EditorBlueprintResources/StandardMacros.IncrementInt` (`self.Index`))
        (:`  `
          (if (> _result (`KismetArrayLibrary.Array_LastIndex` (`self.LofEffectLibrary`)))
            (set `self.Index` 0)))))))

(event `InputAction|SelectLeft`
  (params (Key :type "Key Structure"))
  (:`Pressed`
    ;[1 1 1] 選択メニュー右送り
    (if (`self.IsLogEffectSelect`)
      (bind _result (`/Engine/EditorBlueprintResources/StandardMacros.DecrementInt` (`self.Index`))
        (:`  `
          (if (< _result 0)
            (set `self.Index` (`KismetArrayLibrary.Array_LastIndex` (`self.LofEffectLibrary`)))))))))

(event `InputAction|SelectCancel`
  (params (Key :type "Key Structure"))
  (:`Pressed`
    ;[1 1 1] 効果選択キャンセル
    (set `self.IsLogEffectSelect` false)
    (set `self.Index` 0)
    (`GameplayStatics.SetGlobalTimeDilation` 1.0)
    (for _array_element (`self.SelectWindow`)
      (`Widget.SetVisibility` _array_element "Hidden"))))

(event `Key|E`
  (params (Key :type "Key Structure"))
  ;[1 1 1] やり直し
  (:`Pressed`
    (message `/Game/System/IF_MainGameMode.Undo` (`GameplayStatics.GetGameMode`))))

(fn `F_ShowingSelectMenu`
  (set `self.IsLogEffectSelect` true)
  (for _array_element (`self.SelectWindow`)
    (`Widget.SetVisibility` _array_element "Visible")))

(fn `UserConstructionScript`)