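; Base Paper2D log actor that registers an ID with the game mode and handles its own removal.
; On BeginPlay it requests an ID from the game mode, stores it and exposes it through GetID.
; FDestroyLog hides the sprite, disables collision, notifies the game mode to update its log array and sets a short lifespan for delayed cleanup.
; A separate Destroy event removes the actor immediately.
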(event `self.ReceiveBeginPlay`
  (bind _newparam (message `/Game/System/IF_MainGameMode.SendID` (`GameplayStatics.GetGameMode`)))
  (set `self.ID` _newparam))

(event `/Game/Object/IF_Object.Destroy`
  (`self.K2_DestroyActor`))

(event `/Game/Player/IF_Fire.F_DestroyLog`
  (`SceneComponent.SetVisibility` (`self.PaperSprite`) true false)
  (`self.SetActorEnableCollision` false)
  (message `/Game/System/IF_MainGameMode.Log Array Update` (`GameplayStatics.GetGameMode`))
  (`self.SetLifeSpan` 1.0))

(fn `GetID`
  (returns (ID :type Integer))
  (return (`self.ID`)))

(fn `UserConstructionScript`)