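; BP_ReturnThorn is a thorn trap that falls when the player overlaps its trigger and sends a died message to what it hits.
; The trigger raises projectile gravity; the first hit swaps collision from Box to Cube and, after a delay, a looping timer interpolates it back toward its start.
; On nearing the start, or when the player pawn reports respawning, it notifies its SpawnParent and destroys itself.
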(event `self.ReceiveBeginPlay`
  ;[1 1 1] 初期化
  (`PrimitiveComponent.SetCollisionEnabled` (`self.Cube`) "NoCollision")
  (set `self.StartLocation` (`self.K2_GetActorLocation`)))

(event `self.ReceiveTick`
  (params (DeltaSeconds :type "Float (single-precision)"))
  (bind _isrespawn (message `/Game/Player/IF_Player.F_PlayerIsRespawn` (`GameplayStatics.GetPlayerPawn` 0)))
  (if _isrespawn
    (message `/Game/Gimmick/IF_Gimmick.F_DestroyChild` (`self.SpawnParent`))
    (`self.K2_DestroyActor`)))

(event `self.ReceiveHit`
  (params (MyComp :type "PrimitiveComponent Object Reference") (Other :type "Actor Object Reference") (OtherComp :type "PrimitiveComponent Object Reference") (bSelfMoved :type Boolean) (HitLocation :type "Vector Structure") (HitNormal :type "Vector Structure") (NormalImpulse :type "Vector Structure") (Hit :type "HitResult Structure (by ref)"))
  (if (not (`self.OnHit`))
    (message `/Game/Player/IF_Player.F_Died` Other)
    (set `self.OnHit` true)
    (`PrimitiveComponent.SetCollisionEnabled` (`self.Box`) "NoCollision")
    (`PrimitiveComponent.SetCollisionEnabled` (`self.Cube`) "QueryAndPhysics")
    (`KismetSystemLibrary.Delay` 2.0)
    (`KismetSystemLibrary.K2_SetTimerDelegate` (delegate `ResetLocation`) 0.01 true)))

(event `ResetLocation`
  (`self.K2_SetActorLocation` (`KismetMathLibrary.VInterpTo` (`self.K2_GetActorLocation`) (`self.StartLocation`) (`GameplayStatics.GetWorldDeltaSeconds`) 1.0))
  (if (== (`self.K2_GetActorLocation`) (`self.StartLocation`) :`ErrorTolerance` 2.0)
    (message `/Game/Gimmick/IF_Gimmick.F_DestroyChild` (`self.SpawnParent`))
    (`self.K2_DestroyActor`)))

(event `self.Box1.OnComponentBeginOverlap`
  (params (OverlappedComponent :type "PrimitiveComponent Object Reference") (OtherActor :type "Actor Object Reference") (OtherComp :type "PrimitiveComponent Object Reference") (OtherBodyIndex :type Integer) (bFromSweep :type Boolean) (SweepResult :type "HitResult Structure (by ref)"))
  ;[1 1 1] 落下開始
  (if (== OtherActor (`GameplayStatics.GetPlayerPawn` 0))
    (set `ProjectileMovementComponent.ProjectileGravityScale` 3.0 (`self.ProjectileMovement`))))

(fn `UserConstructionScript`)