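; BP_FallThorn is a falling thorn trap that drops when the player enters its Box1 trigger by raising projectile gravity.
; Anything it hits receives a death message, and actors overlapping Box2 receive a log-destroy message.
; Each tick it polls the player pawn for a respawn message, then destroys itself and notifies its SpawnParent that the child is gone.
; The Cube component's collision is disabled at BeginPlay.
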(event `self.ReceiveBeginPlay`
  (`PrimitiveComponent.SetCollisionEnabled` (`self.Cube`) "NoCollision"))

(event `self.ReceiveTick`
  (params (DeltaSeconds :type "Float (single-precision)"))
  (bind _isrespawn (message `/Game/Player/IF_Player.F_PlayerIsRespawn` (`GameplayStatics.GetPlayerPawn` 0)))
  (if _isrespawn
    (`self.K2_DestroyActor`)
    (message `/Game/Gimmick/IF_Gimmick.F_DestroyChild` (`self.SpawnParent`))))

(event `self.ReceiveHit`
  (params (MyComp :type "PrimitiveComponent Object Reference") (Other :type "Actor Object Reference") (OtherComp :type "PrimitiveComponent Object Reference") (bSelfMoved :type Boolean) (HitLocation :type "Vector Structure") (HitNormal :type "Vector Structure") (NormalImpulse :type "Vector Structure") (Hit :type "HitResult Structure (by ref)"))
  (message `/Game/Player/IF_Player.F_Died` Other))

(event `self.Box1.OnComponentBeginOverlap`
  (params (OverlappedComponent :type "PrimitiveComponent Object Reference") (OtherActor :type "Actor Object Reference") (OtherComp :type "PrimitiveComponent Object Reference") (OtherBodyIndex :type Integer) (bFromSweep :type Boolean) (SweepResult :type "HitResult Structure (by ref)"))
  (if (== OtherActor (`GameplayStatics.GetPlayerPawn` 0))
    (set `ProjectileMovementComponent.ProjectileGravityScale` 5.0 (`self.ProjectileMovement`))))

(event `self.Box2.OnComponentBeginOverlap`
  (params (OverlappedComponent :type "PrimitiveComponent Object Reference") (OtherActor :type "Actor Object Reference") (OtherComp :type "PrimitiveComponent Object Reference") (OtherBodyIndex :type Integer) (bFromSweep :type Boolean) (SweepResult :type "HitResult Structure (by ref)"))
  (message `/Game/Player/IF_Fire.F_DestroyLog` OtherActor))

(fn `UserConstructionScript`)