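; BP_ThreeStageLauncher is a gimmick actor that endlessly fires BP_Shuriken projectiles in bursts of three.
; From BeginPlay, a looping Delay spawns a half-scale shuriken at the location and rotation of one of three Arrow components, selected by an index.
; The index steps through the arrows at a short interval, then resets with a longer pause before the next burst.
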(event `self.ReceiveBeginPlay`
  (bind _output (`|GetArrayItem` (`|MakeArray` (`self.Arrow`) (`self.Arrow1`) (`self.Arrow2`)) (`self.index`)))
  (`KismetSystemLibrary.Delay` (`self.FiringSpan`) :!label _label)
  (`|SpawnActorFromClass` "/Game/Gimmick/BP_Shuriken.BP_Shuriken_C" (`KismetMathLibrary.MakeTransform` (`SceneComponent.K2_GetComponentLocation` _output) (`SceneComponent.K2_GetComponentRotation` _output) (0.5 0.5 0.5)) "Undefined" "OverrideRootScale" null null)
  (if (!= (`self.index`) 2)
    (`/Engine/EditorBlueprintResources/StandardMacros.IncrementInt` (`self.index`)
      (:`  `
        (set `self.FiringSpan` 0.5)
        (goto _label)))
    (else
      (set `self.index` 0)
      (set `self.FiringSpan` 2.0)
      (goto _label))))

(fn `UserConstructionScript`)