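; BP_Shuriken is a projectile gimmick, filed under Launcher, that kills the player character on hit.
; On BeginPlay it applies its initial speed to the ProjectileMovement component and sets its lifespan.
; Any hit destroys it, first sending FDiedMessage if the player was struck.
; Every tick it polls the player pawn's GetMetamoMessage and, when true, zeroes its own time dilation to freeze, with no reset here.
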(event `self.ReceiveTick`
  (params (DeltaSeconds :type "Float (single-precision)"))
  (bind _ismetamo (message `/Game/Player/IF_Player.GetMetamo` (`GameplayStatics.GetPlayerPawn` 0)))
  (if _ismetamo
    (set `self.CustomTimeDilation` 0.0)))

(event `self.ReceiveBeginPlay`
  (set `ProjectileMovementComponent.InitialSpeed` (`self.Initial Speed`) (`self.ProjectileMovement`))
  (`self.SetLifeSpan` (`self.In Lifespan`)))

(event `self.ReceiveHit`
  (params (MyComp :type "PrimitiveComponent Object Reference") (Other :type "Actor Object Reference") (OtherComp :type "PrimitiveComponent Object Reference") (bSelfMoved :type Boolean) (HitLocation :type "Vector Structure") (HitNormal :type "Vector Structure") (NormalImpulse :type "Vector Structure") (Hit :type "HitResult Structure (by ref)"))
  (if (== Other (`GameplayStatics.GetPlayerCharacter` 0))
    (message `/Game/Player/IF_Player.F_Died` Other)
    (`self.K2_DestroyActor`)
    (else
      (`self.K2_DestroyActor`))))

(fn `UserConstructionScript`)