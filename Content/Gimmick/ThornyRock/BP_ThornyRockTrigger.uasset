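; BP_ThornyRockTrigger is a trigger box that starts a thorny rock simulating when the player pawn overlaps it.
; On overlap, it scans every actor implementing IF_ThornyRock, keeping the one with the smallest signed X offset from the player.
; The comparison uses no absolute value, so it selects the lowest-X rock rather than the nearest.
; Only that rock receives FSimulateStartMessage.
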(event `self.Box.OnComponentBeginOverlap`
  (params (OverlappedComponent :type "PrimitiveComponent Object Reference") (OtherActor :type "Actor Object Reference") (OtherComp :type "PrimitiveComponent Object Reference") (OtherBodyIndex :type Integer) (bFromSweep :type Boolean) (SweepResult :type "HitResult Structure (by ref)"))
  (if (== OtherActor (`GameplayStatics.GetPlayerPawn` 0))
    (bind _outactors (`GameplayStatics.GetAllActorsWithInterface` "/Game/Gimmick/ThornyRock/IF_ThornyRock.IF_ThornyRock_C"))
    (for (_array_element _array_index) _outactors
      (if (== _array_index 0)
        (set `self.SimuStartRock` _array_element)
        (elif (< (.x (- (`self.K2_GetActorLocation` _array_element) (`self.K2_GetActorLocation` OtherActor))) (.x (- (`self.K2_GetActorLocation` (`self.SimuStartRock`)) (`self.K2_GetActorLocation` OtherActor))))
          (set `self.SimuStartRock` _array_element))))
    (message `/Game/Gimmick/ThornyRock/IF_ThornyRock.F_SimulateStart` (`self.SimuStartRock`))))

(fn `UserConstructionScript`)