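; BP_ThornyRock is a thorny rock hazard that kills the player on contact by sending a died message.
; Its sphere begins simulating physics when FSimulateStart is called.
; Each tick it polls the player pawn's respawn message, and when true it notifies its SpawnParent through FDestroyChildMessage and destroys itself.
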(event `/Game/Gimmick/ThornyRock/IF_ThornyRock.F_SimulateStart`
  (`PrimitiveComponent.SetSimulatePhysics` (`self.Sphere`) true))

(event `self.ReceiveTick`
  (params (DeltaSeconds :type "Float (single-precision)"))
  (bind _isrespawn (message `/Game/Player/IF_Player.F_PlayerIsRespawn` (`GameplayStatics.GetPlayerPawn` 0)))
  (if _isrespawn
    (message `/Game/Gimmick/IF_Gimmick.F_DestroyChild` (`self.SpawnParent`))
    (`self.K2_DestroyActor`)))

(event `self.ReceiveHit`
  (params (MyComp :type "PrimitiveComponent Object Reference") (Other :type "Actor Object Reference") (OtherComp :type "PrimitiveComponent Object Reference") (bSelfMoved :type Boolean) (HitLocation :type "Vector Structure") (HitNormal :type "Vector Structure") (NormalImpulse :type "Vector Structure") (Hit :type "HitResult Structure (by ref)"))
  (if (== Other (`GameplayStatics.GetPlayerPawn` 0))
    (message `/Game/Player/IF_Player.F_Died` Other)))

(fn `UserConstructionScript`)