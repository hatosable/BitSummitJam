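; BP_FallingFloar_2 is a falling floor gimmick that drops shortly after the player touches it.
; An overlap on Box by the player raises the ProjectileMovement gravity scale after a brief delay, then later messages SpawnParent and destroys the floor.
; A second volume, Box1, acts as a hazard, sending a respawn message to an overlapping player pawn and a destroy-log message to any other actor.
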(event `self.Box.OnComponentBeginOverlap`
  (params (OverlappedComponent :type "PrimitiveComponent Object Reference") (OtherActor :type "Actor Object Reference") (OtherComp :type "PrimitiveComponent Object Reference") (OtherBodyIndex :type Integer) (bFromSweep :type Boolean) (SweepResult :type "HitResult Structure (by ref)"))
  (if (== OtherActor (`GameplayStatics.GetPlayerCharacter` 0))
    (`KismetSystemLibrary.Delay` 0.1)
    (set `ProjectileMovementComponent.ProjectileGravityScale` 3.0 (`self.ProjectileMovement`))
    (`KismetSystemLibrary.Delay` 2.0)
    (message `/Game/Gimmick/IF_Gimmick.F_DestroyChild` (`self.SpawnParent`))
    (`self.K2_DestroyActor`)))

(event `self.Box1.OnComponentBeginOverlap`
  (params (OverlappedComponent :type "PrimitiveComponent Object Reference") (OtherActor :type "Actor Object Reference") (OtherComp :type "PrimitiveComponent Object Reference") (OtherBodyIndex :type Integer) (bFromSweep :type Boolean) (SweepResult :type "HitResult Structure (by ref)"))
  (if (== OtherActor (`GameplayStatics.GetPlayerPawn` 0))
    (message `/Game/Player/IF_Player.F_Respwn` OtherActor)
    (else
      (message `/Game/Player/IF_Fire.F_DestroyLog` OtherActor))))

(fn `UserConstructionScript`)